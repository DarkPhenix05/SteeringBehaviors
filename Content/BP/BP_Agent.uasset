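; Steering-behavior agent that drives a physics cone to seek, flee or wander, drawing debug arrows.
; VisionArea overlaps maintain Objectives; each Tick picks the nearest BP_Target, or wanders toward periodically randomized points without one.
; Box contact relocates the target and switches Seek to Flee until about 1000 units away.
; Behaviors add normalized, scaled steering to velocity; Pursue duplicates Seek and is never called.
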(event OnComponentEndOverlap(VisionArea)
  (params (OverlappedComponent :type Primitive%20Component%20Object%20Reference) (OtherActor :type Actor%20Object%20Reference) (OtherComp :type Primitive%20Component%20Object%20Reference) (OtherBodyIndex :type Integer))
  (bind _returnvalue (Utilities|Set|Remove (Variables|Default|GetObjectives) OtherActor))
  (if _returnvalue
    (Development|PrintString "REMOVED" true true "(R=1.000000,G=0.805385,B=0.000000,A=1.000000)")
    (else
      (Development|PrintString "FALLED TO REMOVE" true true "(R=1.000000,G=0.000000,B=0.000000,A=1.000000)"))))

(event OnComponentBeginOverlap(Box)
  (params (OverlappedComponent :type Primitive%20Component%20Object%20Reference) (OtherActor :type Actor%20Object%20Reference) (OtherComp :type Primitive%20Component%20Object%20Reference) (OtherBodyIndex :type Integer) (bFromSweep :type Boolean) (SweepResult :type Hit%20Result%20Structure%20%28by%20ref%29))
  (bind _asbp_target (Utilities|Casting|CastToBP_Target OtherActor)
    (:then
      (Default|NewLocation _asbp_target)
      (Variables|Default|SetSeeking false))
    (:CastFailed
      (Development|PrintString "Falled Cast - NEW LOCATION" true true "(R=1.000000,G=0.000000,B=0.000000,A=1.000000)"))))

(event OnComponentBeginOverlap(VisionArea)
  (params (OverlappedComponent :type Primitive%20Component%20Object%20Reference) (OtherActor :type Actor%20Object%20Reference) (OtherComp :type Primitive%20Component%20Object%20Reference) (OtherBodyIndex :type Integer) (bFromSweep :type Boolean) (SweepResult :type Hit%20Result%20Structure%20%28by%20ref%29))
  (Utilities|Set|Add (Variables|Default|GetObjectives) OtherActor)
  (Development|PrintString "ADDED" true true "(R=1.000000,G=0.952515,B=0.000000,A=1.000000)"))

(event Custom|UpdateTargetPos
  (bind _asbp_target (Utilities|Casting|CastToBP_Target (Variables|Default|GetTarget))
    (:then
      (bind _return (Default|ReturnPosition _asbp_target))
      (Variables|Default|SetTargetPos _return)
      (Development|PrintString "UPDATE POS" true true "(R=1.000000,G=0.694544,B=0.000000,A=1.000000)"))
    (:CastFailed
      (Development|PrintString "Falled Cast - UPDATE POS" true true "(R=1.000000,G=0.000000,B=0.000000,A=1.000000)"))))

(event Custom|UpdateState
  (CallFunction|FindTarget)
  (if (Variables|Default|GetHaveTarget)
    (CallFunction|UpdateTargetPos)
    (if (and (>= (Math|Vector|VectorLength (Math|Vector|VectorGetAbs (- (Transformation|GetWorldLocation (Variables|Default|GetCone)) (Variables|Default|GetTargetPos)))) 1e+03) (== (Variables|Default|GetSeeking) false))
      (Variables|Default|SetSeeking true))))

(event Custom|FindTarget
  (Variables|Default|SetSmallestDist 9999999.0)
  (Variables|Default|SetHaveTarget false)
  (if (> (Utilities|Set|Length (Variables|Default|GetObjectives)) 0)
    (bind _result (Utilities|Set|ToArray (Variables|Default|GetObjectives)))
    (for _array_element _result
      (bind _asbp_target (Utilities|Casting|CastToBP_Target _array_element)
        (:then
          (bind _return (Default|ReturnPosition _asbp_target))
          (if (< (Math|Float|Absolute(Float) (Math|Vector|VectorLength (- (Transformation|GetWorldLocation (Variables|Default|GetCone)) _return))) (Variables|Default|GetSmallestDist))
            (Variables|Default|SetSmallestDist (Math|Float|Absolute(Float) (Math|Vector|VectorLength (- (Transformation|GetWorldLocation (Variables|Default|GetCone)) _return))))
            (Variables|Default|SetTarget _asbp_target)
            (Variables|Default|SetHaveTarget true)))
        (:CastFailed
          (Development|PrintString "FAILLED TO FIND TARGET" true true "(R=1.000000,G=0.145579,B=0.786394,A=1.000000)"))))
    (if (Variables|Default|GetHaveTarget)
      (Development|PrintString "FOUND TARGET" true true "(R=1.000000,G=0.683000,B=0.000000,A=1.000000)"))))

(event EventBeginPlay
  (Utilities|Set|Clear (Variables|Default|GetObjectives)))

(event EventTick
  (params (DeltaSeconds :type Float%20%28single-precision%29))
  (bind _targetpos (Variables|Default|GetTargetPos))
  (Variables|Default|SetDT DeltaSeconds)
  (CallFunction|UpdateState)
  (if (not (Variables|Default|GetHaveTarget))
    (if (>= (Math|Float|Absolute(Float) (Math|Vector|VectorLength (- (Variables|Default|GetTargetPos) (Transformation|GetWorldLocation (Variables|Default|GetCone))))) 5.0)
      (CallFunction|Wondere true 5.0 1.0 (Variables|Default|GetTargetPos))
      (else
        (Physics|SetPhysicsLinearVelocity (Variables|Default|GetCone) "0, 0, 0" false "None")
        (Development|PrintString "ARRIVED")))
    (elif (Variables|Default|GetSeeking)
      (CallFunction|Seek _targetpos true 5.0)
      (else
        (CallFunction|Flee _targetpos true 5.0)))))

(fn ConstructionScript)

(fn LookatVel
  (bind _cone (Variables|Default|GetCone))
  (bind _currentvel (Variables|Default|GetCurrentVel))
  (bind _returnvalue (Transformation|GetWorldLocation _cone))
  (bind _returnvalue_2 (+ _returnvalue _currentvel))
  (bind _returnvalue_3 (Math|Rotator|FindLookatRotation _returnvalue _returnvalue_2))
  (bind (_roll _pitch _yaw) (Math|Rotator|BreakRotator _returnvalue_3))
  (Transformation|SetWorldRotation _cone (Math|Rotator|MakeRotator _roll (+ _pitch -9e+01) _yaw) false false))

(fn Seek
  (params (DecieredPos :type Vector) (Debug :type Boolean) (SteerMagnitude :type Float%20%28double-precision%29))
  (bind _cone (Variables|Default|GetCone))
  ;[0.6406 0.6375 0 0.5] SETs
  (LocalVariables|Set_DesieredPos DecieredPos)
  (LocalVariables|Set_CurrentVel (Transformation|GetComponentVelocity _cone))
  (LocalVariables|Set_CurrentPos (Transformation|GetWorldLocation _cone))
  (LocalVariables|Set_Debug Debug)
  (LocalVariables|SetSteeringMagnitude SteerMagnitude)
  (Utilities|FlowControl|Sequence
    (:then_0
      ;[0.15 0.15 0.15 0.5] DEBUG
      (if (LocalVariables|Get_Debug)
        (Rendering|Debug|DrawDebugArrow (LocalVariables|Get_CurrentPos) (+ (LocalVariables|Get_CurrentPos) (LocalVariables|Get_CurrentVel)) 3e+01 "(R=0.000000,G=0.864583,B=0.000000,A=0.500000)" 0.0 1.0)))
    (:then_1
      ;[0.09759 0.02315 0.15 0.502] Vector Desiered Vel
      (LocalVariables|SetDesiredVel (- (LocalVariables|Get_DesieredPos) (LocalVariables|Get_CurrentPos))))
    (:then_2
      ;[0.15 0.15 0.15 0.5] DEBUG
      (if (LocalVariables|Get_Debug)
        (Rendering|Debug|DrawDebugArrow (LocalVariables|Get_CurrentPos) (+ (LocalVariables|Get_CurrentPos) (LocalVariables|GetDesiredVel)) 3e+01 "(R=0.097587,G=0.023153,B=0.149960,A=0.500000)" 0.0 1.0)))
    (:then_3
      ;[0.15 0 0.008023 0.502] Steering
      (bind _output_get (LocalVariables|SetSteering (- (+ (LocalVariables|Get_CurrentPos) (LocalVariables|GetDesiredVel)) (+ (LocalVariables|Get_CurrentVel) (LocalVariables|Get_CurrentPos)))))
      ;[0.4896 0.2092 0 0.5] N_Steering
      (bind _output_get_2 (LocalVariables|SetN_Sterring (Math|Vector|Normalize _output_get)))
      ;[0 0.224 0.2008 0.5] Scale Steering
      (LocalVariables|SetFinalSteering (* _output_get_2 (LocalVariables|GetSteeringMagnitude))))
    (:then_4
      ;[0.15 0.15 0.15 0.5] DEBUG
      (if (LocalVariables|Get_Debug)
        (Rendering|Debug|DrawDebugArrow (+ (LocalVariables|Get_CurrentPos) (LocalVariables|Get_CurrentVel)) (+ (+ (LocalVariables|Get_CurrentPos) (LocalVariables|Get_CurrentVel)) (LocalVariables|GetSteering)) 3e+01 "(R=0.149960,G=0.000000,B=0.008023,A=0.500000)" 0.0 1.0)))
    (:then_5
      ;[0.15 0.15 0.15 0.5] DEBUG
      (if (LocalVariables|Get_Debug)
        (Rendering|Debug|DrawDebugArrow (+ (LocalVariables|Get_CurrentPos) (LocalVariables|Get_CurrentVel)) (+ (+ (LocalVariables|Get_CurrentPos) (LocalVariables|Get_CurrentVel)) (* (LocalVariables|GetFinalSteering) (Math|Conversions|ToVector(Float) 1e+01))) 3e+01 "(R=0.000000,G=1.000000,B=0.000000,A=1.000000)" 0.0 1e+01)))
    (:then_6
      ;[0 0.0433 0.3333 0.5] DV + N_Steering
      (bind _output_get_3 (Variables|Default|SetCurrentVel (+ (LocalVariables|Get_CurrentVel) (LocalVariables|GetFinalSteering))))
      ;[0.15 0 0.0679 0.5] AddForce
      (Physics|SetPhysicsLinearVelocity (Variables|Default|GetCone) _output_get_3 false "None")
      (CallFunction|LookatVel))))

(fn Flee
  (params (DecieredPos :type Vector) (Debug :type Boolean) (SteerMagnitude :type Float%20%28double-precision%29))
  (bind _cone (Variables|Default|GetCone))
  ;[0.6406 0.6375 0 0.5] SETs
  (LocalVariables|Set_DesieredPos DecieredPos)
  (LocalVariables|Set_CurrentVel (Transformation|GetComponentVelocity _cone))
  (LocalVariables|Set_CurrentPos (Transformation|GetWorldLocation _cone))
  (LocalVariables|Set_Debug Debug)
  (LocalVariables|SetSteeringMagnitude SteerMagnitude)
  (Utilities|FlowControl|Sequence
    (:then_0
      ;[0.15 0.15 0.15 0.5] DEBUG
      (if (LocalVariables|Get_Debug)
        (Rendering|Debug|DrawDebugArrow (LocalVariables|Get_CurrentPos) (+ (LocalVariables|Get_CurrentPos) (LocalVariables|Get_CurrentVel)) 3e+01 "(R=0.000000,G=0.864583,B=0.000000,A=0.500000)" 0.0 1.0)))
    (:then_1
      ;[0.09759 0.02315 0.15 0.502] Vector Desiered Vel
      (LocalVariables|SetDesiredVel (- (LocalVariables|Get_DesieredPos) (LocalVariables|Get_CurrentPos))))
    (:then_2
      ;[0.15 0.15 0.15 0.5] DEBUG
      (if (LocalVariables|Get_Debug)
        (Rendering|Debug|DrawDebugArrow (LocalVariables|Get_CurrentPos) (+ (LocalVariables|Get_CurrentPos) (LocalVariables|GetDesiredVel)) 3e+01 "(R=0.097587,G=0.023153,B=0.149960,A=0.500000)" 0.0 1.0)))
    (:then_3
      ;[0.15 0 0.008023 0.502] Steering
      (bind _output_get (LocalVariables|SetSteering (- (+ (LocalVariables|Get_CurrentPos) (LocalVariables|GetDesiredVel)) (+ (LocalVariables|Get_CurrentVel) (LocalVariables|Get_CurrentPos)))))
      ;[0.4896 0.2092 0 0.5] N_Steering
      (bind _output_get_2 (LocalVariables|SetN_Sterring (Math|Vector|Normalize _output_get)))
      ;[0 0.224 0.2008 0.5] Scale Steering
      (LocalVariables|SetFinalSteering (* _output_get_2 (* (Math|Conversions|ToVector(Float) -1.0) (LocalVariables|GetSteeringMagnitude)))))
    (:then_4
      ;[0.15 0.15 0.15 0.5] DEBUG
      (if (LocalVariables|Get_Debug)
        (Rendering|Debug|DrawDebugArrow (+ (LocalVariables|Get_CurrentPos) (LocalVariables|Get_CurrentVel)) (+ (+ (LocalVariables|Get_CurrentPos) (LocalVariables|Get_CurrentVel)) (LocalVariables|GetSteering)) 3e+01 "(R=0.149960,G=0.000000,B=0.008023,A=0.500000)" 0.0 1.0)))
    (:then_5
      ;[0.15 0.15 0.15 0.5] DEBUG
      (if (LocalVariables|Get_Debug)
        (Rendering|Debug|DrawDebugArrow (+ (LocalVariables|Get_CurrentPos) (LocalVariables|Get_CurrentVel)) (+ (+ (LocalVariables|Get_CurrentPos) (LocalVariables|Get_CurrentVel)) (* (LocalVariables|GetFinalSteering) (Math|Conversions|ToVector(Float) 1e+01))) 3e+01 "(R=1.000000,G=0.000000,B=0.000000,A=1.000000)" 0.0 1e+01)))
    (:then_6
      ;[0 0.0433 0.3333 0.5] DV + N_Steering
      (bind _output_get_3 (Variables|Default|SetCurrentVel (+ (LocalVariables|Get_CurrentVel) (LocalVariables|GetFinalSteering))))
      ;[0.15 0 0.0679 0.5] AddForce
      (Physics|SetPhysicsLinearVelocity (Variables|Default|GetCone) _output_get_3 false "None")
      (CallFunction|LookatVel))))

(fn Pursue
  (params (DecieredPos :type Vector) (Debug :type Boolean) (SteerMagnitude :type Float%20%28double-precision%29))
  (bind _cone (Variables|Default|GetCone))
  ;[0.6406 0.6375 0 0.5] SETs
  (LocalVariables|Set_DesieredPos DecieredPos)
  (LocalVariables|Set_CurrentVel (Transformation|GetComponentVelocity _cone))
  (LocalVariables|Set_CurrentPos (Transformation|GetWorldLocation _cone))
  (LocalVariables|Set_Debug Debug)
  (LocalVariables|SetSteeringMagnitude SteerMagnitude)
  (Utilities|FlowControl|Sequence
    (:then_0
      ;[0.15 0.15 0.15 0.5] DEBUG
      (if (LocalVariables|Get_Debug)
        (Rendering|Debug|DrawDebugArrow (LocalVariables|Get_CurrentPos) (+ (LocalVariables|Get_CurrentPos) (LocalVariables|Get_CurrentVel)) 3e+01 "(R=0.000000,G=0.864583,B=0.000000,A=0.500000)" 0.0 1.0)))
    (:then_1
      ;[0.09759 0.02315 0.15 0.502] Vector Desiered Vel
      (LocalVariables|SetDesiredVel (- (LocalVariables|Get_DesieredPos) (LocalVariables|Get_CurrentPos))))
    (:then_2
      ;[0.15 0.15 0.15 0.5] DEBUG
      (if (LocalVariables|Get_Debug)
        (Rendering|Debug|DrawDebugArrow (LocalVariables|Get_CurrentPos) (+ (LocalVariables|Get_CurrentPos) (LocalVariables|GetDesiredVel)) 3e+01 "(R=0.097587,G=0.023153,B=0.149960,A=0.500000)" 0.0 1.0)))
    (:then_3
      ;[0.15 0 0.008023 0.502] Steering
      (bind _output_get (LocalVariables|SetSteering (- (+ (LocalVariables|Get_CurrentPos) (LocalVariables|GetDesiredVel)) (+ (LocalVariables|Get_CurrentVel) (LocalVariables|Get_CurrentPos)))))
      ;[0.4896 0.2092 0 0.5] N_Steering
      (bind _output_get_2 (LocalVariables|SetN_Sterring (Math|Vector|Normalize _output_get)))
      ;[0 0.224 0.2008 0.5] Scale Steering
      (LocalVariables|SetFinalSteering (* _output_get_2 (LocalVariables|GetSteeringMagnitude))))
    (:then_4
      ;[0.15 0.15 0.15 0.5] DEBUG
      (if (LocalVariables|Get_Debug)
        (Rendering|Debug|DrawDebugArrow (+ (LocalVariables|Get_CurrentPos) (LocalVariables|Get_CurrentVel)) (+ (+ (LocalVariables|Get_CurrentPos) (LocalVariables|Get_CurrentVel)) (LocalVariables|GetSteering)) 3e+01 "(R=0.149960,G=0.000000,B=0.008023,A=0.500000)" 0.0 1.0)))
    (:then_5
      ;[0.15 0.15 0.15 0.5] DEBUG
      (if (LocalVariables|Get_Debug)
        (Rendering|Debug|DrawDebugArrow (+ (LocalVariables|Get_CurrentPos) (LocalVariables|Get_CurrentVel)) (+ (+ (LocalVariables|Get_CurrentPos) (LocalVariables|Get_CurrentVel)) (* (LocalVariables|GetFinalSteering) (Math|Conversions|ToVector(Float) 1e+01))) 3e+01 "(R=0.000000,G=1.000000,B=0.000000,A=1.000000)" 0.0 1e+01)))
    (:then_6
      ;[0 0.0433 0.3333 0.5] DV + N_Steering
      (bind _output_get_3 (Variables|Default|SetCurrentVel (+ (LocalVariables|Get_CurrentVel) (LocalVariables|GetFinalSteering))))
      ;[0.15 0 0.0679 0.5] AddForce
      (Physics|SetPhysicsLinearVelocity (Variables|Default|GetCone) _output_get_3 false "None")
      (CallFunction|LookatVel))))

(fn Wondere
  (params (Debug :type Boolean) (SteerMagnitude :type Float%20%28double-precision%29) (WaitTime :type Float%20%28double-precision%29) (TargetPosition :type Vector))
  (bind _cone (Variables|Default|GetCone))
  ;[0.6406 0.6375 0 0.5] SETs
  (LocalVariables|Set_DesieredPos TargetPosition)
  (LocalVariables|Set_CurrentVel (Transformation|GetComponentVelocity _cone))
  (LocalVariables|Set_CurrentPos (Transformation|GetWorldLocation _cone))
  (LocalVariables|Set_Debug Debug)
  (LocalVariables|SetSteeringMagnitude SteerMagnitude)
  (LocalVariables|SetWait WaitTime)
  (if (>= (Variables|Default|GetTimerWonder) (LocalVariables|GetWait))
    (Variables|Default|SetTimerWonder 0.0)
    (Variables|Default|SetTargetPos (+ (LocalVariables|Get_CurrentPos) (* (Math|Random|RandomUnitVector) (Math|Conversions|ToVector(Float) (Math|Random|RandomFloatinRange 1e+03 2e+03)))))
    (else
      (Variables|Default|SetTimerWonder (+ (Variables|Default|GetTimerWonder) (Variables|Default|GetDT)))))
  (Utilities|FlowControl|Sequence
    (:then_0
      ;[0.15 0.15 0.15 0.5] DEBUG
      (if (LocalVariables|Get_Debug)
        (Rendering|Debug|DrawDebugArrow (LocalVariables|Get_CurrentPos) (+ (LocalVariables|Get_CurrentPos) (LocalVariables|Get_CurrentVel)) 3e+01 "(R=0.000000,G=0.864583,B=0.000000,A=0.500000)" 0.0 1.0)))
    (:then_1
      ;[0.09759 0.02315 0.15 0.502] Vector Desiered Vel
      (LocalVariables|SetDesiredVel (- (LocalVariables|Get_DesieredPos) (LocalVariables|Get_CurrentPos))))
    (:then_2
      ;[0.15 0.15 0.15 0.5] DEBUG
      (if (LocalVariables|Get_Debug)
        (Rendering|Debug|DrawDebugArrow (LocalVariables|Get_CurrentPos) (+ (LocalVariables|Get_CurrentPos) (LocalVariables|GetDesiredVel)) 3e+01 "(R=0.097587,G=0.023153,B=0.149960,A=0.500000)" 0.0 1.0)))
    (:then_3
      ;[0.15 0 0.008023 0.502] Steering
      (bind _output_get (LocalVariables|SetSteering (- (+ (LocalVariables|Get_CurrentPos) (LocalVariables|GetDesiredVel)) (+ (LocalVariables|Get_CurrentVel) (LocalVariables|Get_CurrentPos)))))
      ;[0.4896 0.2092 0 0.5] N_Steering
      (bind _output_get_2 (LocalVariables|SetN_Sterring (Math|Vector|Normalize _output_get)))
      ;[0 0.224 0.2008 0.5] Scale Steering
      (LocalVariables|SetFinalSteering (* _output_get_2 (LocalVariables|GetSteeringMagnitude))))
    (:then_4
      ;[0.15 0.15 0.15 0.5] DEBUG
      (if (LocalVariables|Get_Debug)
        (Rendering|Debug|DrawDebugArrow (+ (LocalVariables|Get_CurrentPos) (LocalVariables|Get_CurrentVel)) (+ (+ (LocalVariables|Get_CurrentPos) (LocalVariables|Get_CurrentVel)) (LocalVariables|GetSteering)) 3e+01 "(R=0.149960,G=0.000000,B=0.008023,A=0.500000)" 0.0 1.0)))
    (:then_5
      ;[0.15 0.15 0.15 0.5] DEBUG
      (if (LocalVariables|Get_Debug)
        (Rendering|Debug|DrawDebugArrow (+ (LocalVariables|Get_CurrentPos) (LocalVariables|Get_CurrentVel)) (+ (+ (LocalVariables|Get_CurrentPos) (LocalVariables|Get_CurrentVel)) (* (LocalVariables|GetFinalSteering) (Math|Conversions|ToVector(Float) 1e+01))) 3e+01 "(R=0.000000,G=1.000000,B=0.000000,A=1.000000)" 0.0 1e+01)))
    (:then_6
      ;[0 0.0433 0.3333 0.5] DV + N_Steering
      (bind _output_get_3 (Variables|Default|SetCurrentVel (+ (LocalVariables|Get_CurrentVel) (LocalVariables|GetFinalSteering))))
      ;[0.15 0 0.0679 0.5] AddForce
      (Physics|SetPhysicsLinearVelocity (Variables|Default|GetCone) _output_get_3 false "None")
      (CallFunction|LookatVel))))