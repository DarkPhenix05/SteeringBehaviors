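; BP_TargetSpawner is an actor that spawns a configurable number of targets, set by NumberOfTragets, when play begins.
; A counter-driven loop wired back into its branch calls SpawnActor until the count is reached; the spawned class is not specified.
; Locations come from random unit vectors scaled to a fixed radius around the world origin, with absolute Z keeping them at or above zero height.
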(event EventBeginPlay
  (bind _returnvalue (Math|Random|RandomUnitVector))
  (bind _returnvalue_2 (Math|Conversions|ToVector(Float) 5e+03))
  (bind _returnvalue_3 (* _returnvalue _returnvalue_2))
  (Variables|Default|SetCurentTargetCount 0)
  (if (< (Variables|Default|GetCurentTargetCount) (Variables|Default|GetNumberOfTragets)) :!label _label
    (Game|SpawnActorfromClass "/Game/BP/BP_Target.BP_Target_C" (Math|Transform|MakeTransform (Math|Vector|MakeVector (.x _returnvalue_3) (.y _returnvalue_3) (Math|Float|Absolute(Float) (.z _returnvalue_3))) "0, 0, 0" "1.000000,1.000000,1.000000") "Undefined" "MultiplyWithRoot" 0 0)
    (Variables|Default|SetCurentTargetCount (+ (Variables|Default|GetCurentTargetCount) 1))
    (goto _label)))

(fn ConstructionScript)