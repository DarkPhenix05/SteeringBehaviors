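; BP_Target is a target actor whose Sphere component jumps to random positions, exposing its location through ReturnPosition.
; The NewLocation event waits briefly, offsets the Sphere by a random direction and distance, forces Z non-negative with Abs, and prints a debug message.
; BeginPlay caches a BP_Agent reference, which is not used elsewhere here, and the separate NewLocation function taking DT is empty.
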(event Custom|NewLocation
  (bind _returnvalue (Math|Random|RandomFloatinRange 1e+02 1e+03))
  (bind _returnvalue_2 (Math|Random|RandomUnitVector))
  (bind _sphere (Variables|Default|GetSphere))
  (bind _returnvalue_3 (Math|Conversions|ToVector(Float) _returnvalue))
  (bind _returnvalue_4 (Transformation|GetWorldLocation _sphere))
  (bind _returnvalue_5 (* _returnvalue_2 _returnvalue_3))
  (bind _returnvalue_6 (+ _returnvalue_4 _returnvalue_5))
  (Utilities|FlowControl|Delay 0.2)
  (Transformation|SetWorldLocation _sphere (Math|Vector|MakeVector (.x _returnvalue_6) (.y _returnvalue_6) (Math|Float|Absolute(Float) (.z _returnvalue_6))) false false)
  (Development|PrintString "MOVE"))

(event EventBeginPlay
  (bind _returnvalue (Actor|GetActorOfClass "/Game/BP/BP_Agent.BP_Agent_C"))
  (Variables|Default|SetBP_Agent _returnvalue))

(event Collision|EventActorBeginOverlap
  (params (OtherActor :type Actor%20Object%20Reference)))

(event EventTick
  (params (DeltaSeconds :type Float%20%28single-precision%29)))

(fn ConstructionScript)

(fn ReturnPosition
  (return (Transformation|GetWorldLocation (Variables|Default|GetSphere))))

(fn NewLocation
  (params (DT :type Float%20%28double-precision%29)))